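; GodzillaCharacter is a character Blueprint driven by VRPN tracking of the head and hands.
; Each Tick with a valid head position, it sets yaw from head rotation and feeds previous minus current tracked position into forced movement input, using capsule height for Z.
; It then places the left-hand component relative to the updated head-based position.
; The right-hand position is fetched through GetHandPositions but never applied.
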(event EventTick
  (params (DeltaSeconds :type Float%20%28single-precision%29))
  (bind _capsulecomponent (Variables|Default|GetCapsuleComponent))
  (bind _vrpnheadcomponent (Variables|Components|GetVRPNHeadComponent))
  (bind _returnvalue (Transformation|GetWorldLocation _capsulecomponent))
  (bind _transformvector (Variables|/Script/Godzilla.VRPNComponent|GetTransformVector _vrpnheadcomponent))
  (bind (_x _y) (Math|Vector|BreakVector _transformvector))
  (bind _z (Math|Vector|BreakVector _returnvalue))
  (bind _returnvalue_2 (Math|Vector|MakeVector _x _y _z))
  (if (AI|IsValidAILocation _transformvector)
    (Transformation|SetActorRotation (Math|Rotator|MakeRotator 0.0 0.0 (.Yaw (Math|Rotator|BreakRotator (Variables|/Script/Godzilla.VRPNComponent|GetRotationMatrix _vrpnheadcomponent)))))
    (Pawn|Input|AddMovementInput (- (Variables|Default|GetOldPos) _returnvalue_2) 1.0 true)
    (bind _output_get (Variables|Default|SetOldPos _returnvalue_2))
    (bind _handlvecout (CallFunction|GetHandPositions))
    (Transformation|SetRelativeLocation (Variables|Components|GetVRPNHandLComponent) (- _handlvecout _output_get) false false)))

(fn ConstructionScript
  (Variables|Default|SetOldPos "0, 0, 0"))

(fn GetHandPositions
  (return (Variables|/Script/Godzilla.VRPNComponent|GetTransformVector (Variables|Components|GetVRPNHandRComponent)) (Variables|/Script/Godzilla.VRPNComponent|GetTransformVector (Variables|Components|GetVRPNHandLComponent))))